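; Placeable spot light actor that adds a visible volumetric beam to a standard spot light.
; The construction script copies exposed variables onto a custom VolumetricSpotLight component, setting intensity, color, attenuation and cone angles.
; It also sets the beam's static mesh, material, intensity, light shift, edge falloff and added angle.
; All setup happens at construction; the event graph has no active logic.
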(fn `UserConstructionScript`
  (bind _volumetricspotlight (`self.VolumetricSpotLight`))
  (`LightComponent.SetIntensity` _volumetricspotlight (`self.Light Intensity`))
  (`LightComponent.SetLightColor` _volumetricspotlight (`self.Light Color`) true)
  (`LocalLightComponent.SetAttenuationRadius` _volumetricspotlight (`self.Light Attenuation Radius`))
  (`SpotLightComponent.SetOuterConeAngle` _volumetricspotlight (`self.Light Outer Cone Angle`))
  (`SpotLightComponent.SetInnerConeAngle` _volumetricspotlight (`self.Light Inner Cone Angle`))
  (`VolumetricSpotLightComponent.SetVolumetricStaticMesh` _volumetricspotlight (`self.Volumetric Static Mesh`))
  (`VolumetricSpotLightComponent.SetVolumetricMaterial` _volumetricspotlight (`self.Volumetric Material`))
  (`VolumetricSpotLightComponent.SetVolumetricBeamIntensity` _volumetricspotlight (`self.Volumetric Intensity`))
  (`VolumetricSpotLightComponent.SetVolumetricLightShift` _volumetricspotlight (`self.Volumetric Light Shift`))
  (`VolumetricSpotLightComponent.SetVolumetricEdgeFalloffPower` _volumetricspotlight (`self.Volumetric Edge Falloff Power`))
  (`VolumetricSpotLightComponent.SetVolumetricAddAngle` _volumetricspotlight (`self.Volumetric Add Angle`)))